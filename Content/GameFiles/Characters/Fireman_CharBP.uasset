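; Fireman player character Blueprint that adds jetpack flight, triggered by pressing jump while falling with fuel left.
; Flight switches to flying movement and loops delayed upward input while the key is held, with fuel, tuning and exhaust delegated to the child-actor Jetpack.
; Releasing or emptying fuel drops into falling with boosted air control until landing restores walking and sprinting.
; It also drives flight sound, altitude widget fades and an out-of-fuel HUD animation.
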(event Custom|Play%20jetpack%20sound
  ;[1 0.09196 0] JETPACK
  ;;[0 0 0] Jetpack sounds
  (Audio|PlaySound2D "/Game/GameFiles/Jetpack/JetpackFlightSound.JetpackFlightSound" 1.0 1.0 0.0 0 0 :!label _label)
  (Utilities|FlowControl|Delay 0.1)
  (if (Class|NavMovementComponent|IsFlying (Variables|Character|GetCharacterMovement))
    (goto _label)))

(event Custom|Stop%20flying
  ;[1 0.09196 0] JETPACK
  ;;[0 0 0] Adds movment input in up direction with delay if still using jetpack
  ;;[0 0 0] Stop fuel from decreasing
  (Default|StopDepletion (Variables|/Game/GameFiles/Jetpack/Jetpack_Actor.Jetpack_Actor_C|GetJetpackValues_ActorComponent (CallFunction|AcessJetpack)))
  ;;[0 0 0] If not holding down jetpack flight key, then go to falling movement and reset rotation variables
  (Pawn|Components|CharacterMovement|SetMovementMode (Variables|Character|GetCharacterMovement) "MOVE_Falling" 0)
  (Variables|Default|SetAiming? false)
  (Variables|/Script/Engine.CharacterMovementComponent|SetbOrientRotationToMovement (Variables|Character|GetCharacterMovement) false)
  (Variables|Default|SetbUseControllerRotationYaw true)
  ;;[0 0 0] Makes the jet particle hidden
  (Default|ExhaustParticleSet (CallFunction|AcessJetpack) false)
  ;;[0 0 0] Setting animation far falling with jetpack and leaning
  (bind _asfireman_anim_bp (Utilities|Casting|CastToFireman_AnimBP (CallFunction|GetPlayerAnimInstance)))
  (Variables|/Game/GameFiles/Characters/Animations/Fireman_AnimBP.Fireman_AnimBP_C|SetFalling%20from%20jetpack _asfireman_anim_bp true)
  ;;[0 0 0] Over rides air control when falling from jetpack for more fluid and accurate controlling
  (Default|InitializeFallingValues (CallFunction|AcessJetpack))
  (Variables|/Script/Engine.CharacterMovementComponent|SetAirControl (Variables|Character|GetCharacterMovement) 1.0))

(event Custom|Fade%20in%20altitude%20level%20widget
  ;[1 0.09196 0] JETPACK
  ;;[0 0 0] Fading in and out altitude level widget
  (bind _altitude_level_widget_ref (Variables|Default|GetAltitude%20Level%20widget%20ref)
    (:then
      (Widget|RemovefromParent _altitude_level_widget_ref))
    (:else
      _))
  (bind _returnvalue (UserInterface|CreateWidget "/Game/GameFiles/Widgets/AltitudeLevel/AltitudeLevel_UI.AltitudeLevel_UI_C"))
  (bind _output_get (Variables|Default|SetAltitude%20Level%20widget%20ref _returnvalue))
  (UserInterface|Viewport|AddtoViewport _output_get 0)
  (bind _value (Timeline|Fade%20in%20timeline Play)
    (:Update
      (Variables|Default|GetAltitude%20Level%20widget%20ref
        (:then
          (Widget|SetRenderOpacity (Variables|/Game/GameFiles/Widgets/AltitudeLevel/AltitudeLevel_UI.AltitudeLevel_UI_C|GetMaster _output_get) _value))
        (:else)))
    (:Finished
      (bind _altitude_level_widget_ref_2 (Variables|Default|GetAltitude%20Level%20widget%20ref)
        (:then
          (if (< (Class|Widget|GetRenderOpacity (Variables|/Game/GameFiles/Widgets/AltitudeLevel/AltitudeLevel_UI.AltitudeLevel_UI_C|GetMaster _output_get)) 1.0)
            (Widget|RemovefromParent _altitude_level_widget_ref_2)))
        (:else)))))

(event Custom|Fade%20out%20widget
  ;[1 0.09196 0] JETPACK
  ;;[0 0 0] Fading in and out altitude level widget
  (bind _value (Timeline|Fade%20in%20timeline Reverse)
    (:Update
      (Variables|Default|GetAltitude%20Level%20widget%20ref
        (:then
          (Widget|SetRenderOpacity (Variables|/Game/GameFiles/Widgets/AltitudeLevel/AltitudeLevel_UI.AltitudeLevel_UI_C|GetMaster (stale Custom|Fade%20in%20altitude%20level%20widget _output_get)) _value))
        (:else)))
    (:Finished
      (bind _altitude_level_widget_ref (Variables|Default|GetAltitude%20Level%20widget%20ref)
        (:then
          (if (< (Class|Widget|GetRenderOpacity (Variables|/Game/GameFiles/Widgets/AltitudeLevel/AltitudeLevel_UI.AltitudeLevel_UI_C|GetMaster (stale Custom|Fade%20in%20altitude%20level%20widget _output_get))) 1.0)
            (Widget|RemovefromParent _altitude_level_widget_ref)))
        (:else)))))

(event EventBeginPlay
  (|CallParentFunction))

(event Collision|EventActorBeginOverlap
  (params (OtherActor :type Actor%20Object%20Reference)))

(event EventAddingFuel
  (params (Amount :type Float%20%28single-precision%29))
  ;[1 0.09196 0] JETPACK
  ;;[0 0 0] Adding fuel on pickup
  (Default|AddFuel (Variables|/Game/GameFiles/Jetpack/Jetpack_Actor.Jetpack_Actor_C|GetJetpackValues_ActorComponent (CallFunction|AcessJetpack)) Amount))

(event EventOnLanded
  (params (Hit :type Hit%20Result%20Structure%20%28by%20ref%29))
  (bind _charactermovement (Variables|Character|GetCharacterMovement))
  ;[1 0.09196 0] JETPACK
  ;;[0 0 0] On landed
  (Utilities|FlowControl|Sequence
    (:then_0
      (bind _asfireman_anim_bp (Utilities|Casting|CastToFireman_AnimBP (CallFunction|GetPlayerAnimInstance)))
      (Variables|/Game/GameFiles/Characters/Animations/Fireman_AnimBP.Fireman_AnimBP_C|SetFalling%20from%20jetpack _asfireman_anim_bp false)
      (Variables|/Script/Engine.CharacterMovementComponent|SetAirControl (Variables|Character|GetCharacterMovement) 0.2)
      (Variables|Default|SetbUseControllerRotationYaw false)
      (Variables|/Script/Engine.CharacterMovementComponent|SetbOrientRotationToMovement _charactermovement true)
      (Variables|/Script/Engine.CharacterMovementComponent|SetbUseControllerDesiredRotation _charactermovement false))
    (:then_1
      (CallFunction|OnLandedEvent)
      (Variables|/Script/Engine.CharacterMovementComponent|SetMaxWalkSpeed (Variables|Character|GetCharacterMovement) (Math|Float|SelectFloat (Variables|Default|GetSprint%20speed) (Variables|Default|GetWalking%20Speed) (Variables|Default|GetIs%20Sprinting)))
      (CallFunction|FadeOutWidget)
      ;;;[0 0 0] Allows sprinting
      (Variables|Default|SetCan%20sprint? true))))

(event Input|ActionEvents|InputActionJump
  (params (Key :type Key%20Structure :default "None"))
  (bind _charactermovement (Variables|Character|GetCharacterMovement))
  ;[1 0.09196 0] JETPACK
  (:Pressed
    (Variables|Default|SetJetpack%20input%20key Key)
    ;;[0 0 0] Only use jetpack if falling
    (if (AI|Components|NavMovement|IsFalling (Variables|Character|GetCharacterMovement))
      (if (Default|CheckHasFuel (Variables|/Game/GameFiles/Jetpack/Jetpack_Actor.Jetpack_Actor_C|GetJetpackValues_ActorComponent (CallFunction|AcessJetpack)))
        ;;[0 0 0] Sets movement mode to flying and variables set to rotate character correctly
        (Variables|Default|SetAiming%20Rotation%20Interp%20Speed 8.0)
        (Pawn|Components|CharacterMovement|SetMovementMode (Variables|Character|GetCharacterMovement) "MOVE_Flying" 0)
        (Variables|Default|SetAiming? true)
        (Variables|/Script/Engine.CharacterMovementComponent|SetbOrientRotationToMovement _charactermovement false)
        (Variables|/Script/Engine.CharacterMovementComponent|SetbUseControllerDesiredRotation _charactermovement true)
        ;;[0 0 0] Sets flying speed values
        (bind (_speed _acceleration _thrust_delay) (Default|InitializeValues (CallFunction|AcessJetpack)))
        (Variables|/Script/Engine.CharacterMovementComponent|SetMaxFlySpeed _charactermovement _speed)
        (Variables|/Script/Engine.CharacterMovementComponent|SetMaxAcceleration _charactermovement _acceleration)
        ;;[0 0 0] Makes the jet particle visible
        (Default|ExhaustParticleSet (CallFunction|AcessJetpack) true)
        ;;[0 0 0] Adds movment input in up direction with delay if still using jetpack
        (Utilities|FlowControl|Sequence
          (:then_0
            (if (Default|CheckHasFuel (Variables|/Game/GameFiles/Jetpack/Jetpack_Actor.Jetpack_Actor_C|GetJetpackValues_ActorComponent (CallFunction|AcessJetpack))) :!label _label
              (Pawn|Input|AddMovementInput (Math|Vector|GetUpVector (Math|Rotator|MakeRotator 0.0 0.0 (.yaw (Pawn|GetControlRotation :!class /Script/Engine.Pawn)))) 1.0 false)
              (if (Game|Player|IsInputKeyDown (Game|GetPlayerController 0) (Variables|Default|GetJetpack%20input%20key))
                (Utilities|FlowControl|Sequence
                  (:then_1
                    (Utilities|FlowControl|Delay _thrust_delay)
                    (goto _label)))
                (else
                  ;;[0 0 0] Stop fuel from decreasing
                  (Default|StopDepletion (Variables|/Game/GameFiles/Jetpack/Jetpack_Actor.Jetpack_Actor_C|GetJetpackValues_ActorComponent (CallFunction|AcessJetpack)))
                  ;;[0 0 0] If not holding down jetpack flight key, then go to falling movement and reset rotation variables
                  (Pawn|Components|CharacterMovement|SetMovementMode (Variables|Character|GetCharacterMovement) "MOVE_Falling" 0)
                  (Variables|Default|SetAiming? false)
                  (Variables|/Script/Engine.CharacterMovementComponent|SetbOrientRotationToMovement (Variables|Character|GetCharacterMovement) false)
                  (Variables|Default|SetbUseControllerRotationYaw true)
                  ;;[0 0 0] Makes the jet particle hidden
                  (Default|ExhaustParticleSet (CallFunction|AcessJetpack) false)
                  ;;[0 0 0] Setting animation far falling with jetpack and leaning
                  (bind _asfireman_anim_bp (Utilities|Casting|CastToFireman_AnimBP (CallFunction|GetPlayerAnimInstance)))
                  (Variables|/Game/GameFiles/Characters/Animations/Fireman_AnimBP.Fireman_AnimBP_C|SetFalling%20from%20jetpack _asfireman_anim_bp true)
                  ;;[0 0 0] Over rides air control when falling from jetpack for more fluid and accurate controlling
                  (Default|InitializeFallingValues (CallFunction|AcessJetpack))
                  (Variables|/Script/Engine.CharacterMovementComponent|SetAirControl (Variables|Character|GetCharacterMovement) 1.0)))
              (else
                ;;[0 0 0] If fuel finished, stop flying
                (CallFunction|StopFlying)
                (|Ranoutoffuelwidgetanimation))))
          (:then_1
            ;;[0 0 0] Sounds
            (CallFunction|PlayJetpackSound)
            (Utilities|FlowControl|Sequence
              (:then_0
                ;;[0 0 0] Stops sprinting if currently sprinting
                (if (Variables|Default|GetIs%20Sprinting)
                  (CallFunction|StopSprinting)))
              (:then_1
                ;;[0 0 0] Begins depletion of fuel
                (Default|BeginFuelDepletion (Variables|/Game/GameFiles/Jetpack/Jetpack_Actor.Jetpack_Actor_C|GetJetpackValues_ActorComponent (CallFunction|AcessJetpack)))
                ;;[0 0 0] Prevents sprinting
                (Variables|Default|SetCan%20sprint? false)
                (CallFunction|FadeinAltitudeLevelWidget)))))))))

(fn ConstructionScript
  (bind _asjetpack_actor (CallFunction|AcessJetpack))
  (bind _jetpackvalues_actorcomponent (Variables|/Game/GameFiles/Jetpack/Jetpack_Actor.Jetpack_Actor_C|GetJetpackValues_ActorComponent _asjetpack_actor))
  (|CallParentFunction)
  (Variables|/Game/GameFiles/Jetpack/JetpackValues_ActorComponent.JetpackValues_ActorComponent_C|SetJetpack%20Current%20fuel _jetpackvalues_actorcomponent (Variables|/Game/GameFiles/Jetpack/JetpackValues_ActorComponent.JetpackValues_ActorComponent_C|GetJetpack%20max%20fuel _jetpackvalues_actorcomponent)))

(fn AcessJetpack
  (return (.AsJetpack%20Actor (Utilities|Casting|CastToJetpack_Actor (Variables|/Script/Engine.ChildActorComponent|GetChildActor (Variables|Default|GetJetpack))))))

(fn CheckifFuelIsMaxed
  (bind _asjetpack_actor (CallFunction|AcessJetpack))
  (bind _jetpackvalues_actorcomponent (Variables|/Game/GameFiles/Jetpack/Jetpack_Actor.Jetpack_Actor_C|GetJetpackValues_ActorComponent _asjetpack_actor))
  (return (not (< (Variables|/Game/GameFiles/Jetpack/JetpackValues_ActorComponent.JetpackValues_ActorComponent_C|GetJetpack%20Current%20fuel _jetpackvalues_actorcomponent) (Variables|/Game/GameFiles/Jetpack/JetpackValues_ActorComponent.JetpackValues_ActorComponent_C|GetJetpack%20max%20fuel _jetpackvalues_actorcomponent)))))

(fn GetJetpackFuel
  (bind _asjetpack_actor (CallFunction|AcessJetpack))
  (bind _jetpackvalues_actorcomponent (Variables|/Game/GameFiles/Jetpack/Jetpack_Actor.Jetpack_Actor_C|GetJetpackValues_ActorComponent _asjetpack_actor))
  (return (Variables|/Game/GameFiles/Jetpack/JetpackValues_ActorComponent.JetpackValues_ActorComponent_C|GetJetpack%20Current%20fuel _jetpackvalues_actorcomponent) (Variables|/Game/GameFiles/Jetpack/JetpackValues_ActorComponent.JetpackValues_ActorComponent_C|GetJetpack%20max%20fuel _jetpackvalues_actorcomponent)))

(fn GetValueAboveGround
  (return (Variables|Default|GetWidget%20translation%20for%20height) (Variables|Default|GetDistance%20above%20ground)))